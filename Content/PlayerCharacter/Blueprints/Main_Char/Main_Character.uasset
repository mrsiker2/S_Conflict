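; Player character for a networked shooter, switching between travel mode and battle mode with camera zoom and speed changes.
; Battle mode enables kinetic fire with indexed spread, energy fire and reloading rockets; travel mode regenerates HP, armor and energy.
; Typed projectile damage splits across armor and HP, forces battle mode when travelling, and swaps material on death.
; Inputs relay through server-then-all events, and swept movement slides along blocking surfaces.
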(event Custom|Death_Call_All
  ;[1 1 1] Получение урона и смерть
  (Rendering|Material|SetMaterial (Variables|Default|GetStaticMesh) 0 "/Game/TwinStick/Meshes/OrangeMaterial.OrangeMaterial"))

(event Custom|Refresh_Q
  ;[1 1 1] Активация енергитических выстрелов
  (Utilities|FlowControl|Delay 2.0)
  (Utilities|FlowControl|DoOnce false) ; enters at Reset
)

(event Custom|InmputFireRight_For_Server
  (params (NewParam :type Float%20%28single-precision%29))
  ;[1 1 1] Стрельба
  (CallFunction|InmputFireRightforAll NewParam))

(event Custom|InmputFireRight_For_All
  (params (NewParam :type Float%20%28single-precision%29))
  ;[1 1 1] Стрельба
)

(event Custom|Switch_Fire_type_Call_Server
  ;[1 1 1] Активация енергитических выстрелов
  (CallFunction|SwitchFireTypeCallAll))

(event Custom|Switch_Fire_type_Call_All
  ;[1 1 1] Активация енергитических выстрелов
  (Utilities|FlowControl|DoOnce false
    (:Completed
      (Utilities|FlowControl|FlipFlop
        (:A
          (Variables|Default|SetCanFire false)
          (Variables|Speed|SetMoveSpeed (Variables|Speed|GetMove_Speed_Zero))
          (Utilities|FlowControl|Delay 2.0)
          (Variables|Default|SetEnergy_Fire_Activate? true)
          (Variables|Default|SetCanFire true)
          (Variables|Speed|SetMoveSpeed (Variables|Speed|GetMove_Speed_Battle_Mode)))
        (:B
          (Variables|Default|SetCanFire false)
          (Variables|Speed|SetMoveSpeed (Variables|Speed|GetMove_Speed_Zero))
          (Utilities|FlowControl|Delay 2.0)
          (Variables|Default|SetEnergy_Fire_Activate? false)
          (Variables|Default|SetCanFire true)
          (Variables|Speed|SetMoveSpeed (Variables|Speed|GetMove_Speed_Battle_Mode))))
      (CallFunction|RefreshQ))))

(event Custom|Auto_Switch_Fire_Type
  ;[1 1 1] Активация енергитических выстрелов
  (CallFunction|SwitchFireTypeCallServer))

(event Custom|Auto_Swap_Battle_Mode
  ;[1 1 1] Смена тревел/батл мода
  (CallFunction|SwapBattleModeCallServer))

(event Custom|Swap_Battle_Mode_Call_Server
  ;[1 1 1] Смена тревел/батл мода
  (CallFunction|SwapBattleModeCallAll))

(event Custom|Swap_Battle_Mode_Call_All
  ;[1 1 1] Смена тревел/батл мода
  (Utilities|FlowControl|DoOnce false
    (:Completed
      (Utilities|FlowControl|FlipFlop
        (:A
          (Variables|Speed|SetMoveSpeed (Variables|Speed|GetMove_Speed_Zero))
          (bind _newtrack_0 (Timeline|Camera_Battle_Mode_Activate ReverseFromEnd)
            (:Update
              (Variables|/Script/Engine.SpringArmComponent|SetTargetArmLength (Variables|Default|GetSpringArm) _newtrack_0))
            (:Finished
              (Variables|Speed|SetMoveSpeed (Variables|Speed|GetMove_Speed_Battle_Mode))
              (Variables|Default|SetBattle_Mode_Activate? true)
              (CallFunction|RefreshSwapBattleMode :!label _label))))
        (:B
          (Variables|Default|SetBattle_Mode_Activate? false)
          (Variables|Speed|SetMoveSpeed (Variables|Speed|GetMove_Speed_Zero))
          (bind _newtrack_0_2 (Timeline|Camera_Battle_Mode_DeActivate PlayFromStart)
            (:Update
              (Variables|/Script/Engine.SpringArmComponent|SetTargetArmLength (Variables|Default|GetSpringArm) _newtrack_0_2))
            (:Finished
              (Variables|Speed|SetMoveSpeed (Variables|Speed|GetMove_Speed_Trevel_Mode))
              (CallFunction|StartRegen)
              (goto _label))))))))

(event Custom|Refresh_Swap_Battle_Mode
  ;[1 1 1] Смена тревел/батл мода
  (Utilities|FlowControl|DoOnce false) ; enters at Reset
)

(event Custom|CustomEvent_0
  (CallFunction|CustomEvent1))

(event Custom|Event_On_Possesed_call_Server
  ;[1 1 1] Записать владельца
  (CallFunction|EventonPossesedCallAll))

(event Custom|CustomEvent_1
  (Development|PrintString (Utilities|String|ToString(Integer) (Variables|Default|GetCharacter_Number))))

(event Custom|Fire_Rocket_For_Server
  ;[1 1 1] Rocket
  (CallFunction|FireRocketforAll))

(event Custom|Fire_Rocket_For_All
  ;[1 1 1] Rocket
  (Utilities|FlowControl|DoOnce false :!label _label
    (:Completed
      (CallFunction|ShootRocket)
      (Development|PrintString (Utilities|String|ToString(Integer) (Variables|Rocket_Weapon|GetCurrent_Value_Rockets)))
      (Utilities|FlowControl|Delay 0.2)
      (CallFunction|StartReloadRocket)
      (goto _label Reset))))

(event Custom|Start_Reload_Rocket
  ;[1 1 1] Rocket
  (Utilities|FlowControl|DoOnce false :!label _label
    (:Completed
      (Utilities|FlowControl|Delay (Variables|RocketWeapon|GetRocket_Reload) :!label _label_2)
      (Variables|Rocket_Weapon|SetCurrent_Value_Rockets (+ (Variables|Rocket_Weapon|GetCurrent_Value_Rockets) 1))
      (if (< (Variables|Rocket_Weapon|GetCurrent_Value_Rockets) (Variables|Rocket_Weapon|GetMax_Value_Rockets))
        (goto _label_2)
        (else
          (goto _label Reset))))))

(event Custom|Refresh_Energy
  ;[1 1 1] Регенерация статов
  (Utilities|FlowControl|DoOnce false :!label _label
    (:Completed
      (if (Variables|Default|GetBattle_Mode_Activate?) :!label _label_2
        (goto _label Reset)
        (elif (< (Variables|Ship_Stats|GetCurrent_Energy) (Variables|Ship_Stats|GetMax_Energy))
          (Utilities|FlowControl|Delay 0.2)
          (Variables|Ship_Stats|SetCurrent_Energy (+ (Variables|Ship_Stats|GetCurrent_Energy) (Variables|Ship_Stats|GetEnergy_Regen)))
          (goto _label_2)
          (else
            (goto _label Reset)))))))

(event Custom|Refresh_Shield
  ;[1 1 1] Регенерация статов
  (Utilities|FlowControl|DoOnce false :!label _label
    (:Completed
      (if (Variables|Default|GetBattle_Mode_Activate?) :!label _label_2
        (goto _label Reset)
        (elif (< (Variables|Ship_Stats|GetCurrent_Armor) (Variables|Ship_Stats|GetMax_armor))
          (Utilities|FlowControl|Delay 0.2)
          (Variables|Ship_Stats|SetCurrent_Armor (+ (Variables|Ship_Stats|GetCurrent_Armor) (Variables|Ship_Stats|GetArmor_Regen)))
          (goto _label_2)
          (else
            (goto _label Reset)))))))

(event Custom|Refresh_HP
  ;[1 1 1] Регенерация статов
  (Utilities|FlowControl|DoOnce false :!label _label
    (:Completed
      (if (Variables|Default|GetBattle_Mode_Activate?) :!label _label_2
        (goto _label Reset)
        (elif (< (Variables|Ship_Stats|GetCurrent_HP) (Variables|Ship_Stats|GetMax_HP))
          (Utilities|FlowControl|Delay 0.2)
          (Variables|Ship_Stats|SetCurrent_HP (+ (Variables|Ship_Stats|GetCurrent_HP) (Variables|Ship_Stats|GetHP_Regen)))
          (goto _label_2)
          (else
            (goto _label Reset)))))))

(event Custom|Start_Regen
  ;[1 1 1] Регенерация статов
  (CallFunction|RefreshEnergy)
  (CallFunction|RefreshShield)
  (CallFunction|RefreshHP))

(event Custom|Take_Damage_In_Travel_Mode
  ;[1 1 1] Смена тревел/батл мода
  (Variables|Default|SetBattle_Mode_Activate? true)
  (Variables|Speed|SetMoveSpeed (Variables|Speed|GetMove_Speed_Zero))
  (Utilities|FlowControl|Delay 2.0)
  (CallFunction|SwapBattleModeCallServer))

(event Custom|Event_On_Possesed_call_All
  ;[1 1 1] Записать владельца
  (bind _asplayer_controller_1 (Utilities|Casting|CastToPlayerController1 (stale EventPossessed NewController)))
  (Variables|Default|SetAs%20Player%20Controller%201_REF _asplayer_controller_1)
  (Variables|Default|SetPlayer_Number (Variables|Default|GetCharacter_Number)))

(event Custom|Move_forward_Call_Server
  (params (Axis :type Float%20%28single-precision%29))
  ;[1 1 1] Передвижение
  (CallFunction|MuveForwardCallAll Axis))

(event Custom|Muve_Forward_Call_All
  (params (Axis :type Float%20%28single-precision%29))
  ;[1 1 1] Передвижение
  (if (> (Math|Vector|VectorLength (* (Math|Vector|ClampVectorSize (Math|Vector|MakeVector Axis (stale Custom|Muve_Right_Call_All Axis) 0.0) 0.0 1.0) (* (Utilities|Time|GetWorldDeltaSeconds) (Variables|Speed|GetMoveSpeed)))) 0.0)
    (Transformation|SetWorldRotation (Variables|Default|GetStaticMesh) (Math|Interpolation|RInterpTo (Transformation|GetWorldRotation (Variables|Default|GetStaticMesh)) (Math|Conversions|RotationFromXVector (* (Math|Vector|ClampVectorSize (Math|Vector|MakeVector Axis (stale Custom|Muve_Right_Call_All Axis) 0.0) 0.0 1.0) (* (Utilities|Time|GetWorldDeltaSeconds) (Variables|Speed|GetMoveSpeed)))) (Utilities|Time|GetWorldDeltaSeconds) 5.0) false false)
    (bind _sweephitresult (Transformation|AddActorWorldOffset (* (Math|Vector|ClampVectorSize (Math|Vector|MakeVector Axis (stale Custom|Muve_Right_Call_All Axis) 0.0) 0.0 1.0) (* (Utilities|Time|GetWorldDeltaSeconds) (Variables|Speed|GetMoveSpeed))) true))
    (if (.bBlockingHit (Collision|BreakHitResult _sweephitresult))
      (Transformation|AddActorWorldOffset (* (Math|Vector|ProjectVectorontoPlane (* (Math|Vector|ClampVectorSize (Math|Vector|MakeVector Axis (stale Custom|Muve_Right_Call_All Axis) 0.0) 0.0 1.0) (* (Utilities|Time|GetWorldDeltaSeconds) (Variables|Speed|GetMoveSpeed))) (Math|Vector|Normalize (Math|Vector|MakeVector (.X (Math|Vector|BreakVector (.Normal (Collision|BreakHitResult _sweephitresult)))) (.Y (Math|Vector|BreakVector (.Normal (Collision|BreakHitResult _sweephitresult)))) 0.0))) (- 1.0 (.Time (Collision|BreakHitResult _sweephitresult)))) true))))

(event Custom|Muve_Right_Call_Server
  (params (Axis :type Float%20%28single-precision%29))
  ;[1 1 1] Передвижение
  (CallFunction|MuveRightCallAll Axis))

(event Custom|Muve_Right_Call_All
  (params (Axis :type Float%20%28single-precision%29))
  ;[1 1 1] Передвижение
  (if (> (Math|Vector|VectorLength (* (Math|Vector|ClampVectorSize (Math|Vector|MakeVector (stale Custom|Muve_Forward_Call_All Axis) Axis 0.0) 0.0 1.0) (* (Utilities|Time|GetWorldDeltaSeconds) (Variables|Speed|GetMoveSpeed)))) 0.0)
    (Transformation|SetWorldRotation (Variables|Default|GetStaticMesh) (Math|Interpolation|RInterpTo (Transformation|GetWorldRotation (Variables|Default|GetStaticMesh)) (Math|Conversions|RotationFromXVector (* (Math|Vector|ClampVectorSize (Math|Vector|MakeVector (stale Custom|Muve_Forward_Call_All Axis) Axis 0.0) 0.0 1.0) (* (Utilities|Time|GetWorldDeltaSeconds) (Variables|Speed|GetMoveSpeed)))) (Utilities|Time|GetWorldDeltaSeconds) 5.0) false false)
    (bind _sweephitresult (Transformation|AddActorWorldOffset (* (Math|Vector|ClampVectorSize (Math|Vector|MakeVector (stale Custom|Muve_Forward_Call_All Axis) Axis 0.0) 0.0 1.0) (* (Utilities|Time|GetWorldDeltaSeconds) (Variables|Speed|GetMoveSpeed))) true))
    (if (.bBlockingHit (Collision|BreakHitResult _sweephitresult))
      (Transformation|AddActorWorldOffset (* (Math|Vector|ProjectVectorontoPlane (* (Math|Vector|ClampVectorSize (Math|Vector|MakeVector (stale Custom|Muve_Forward_Call_All Axis) Axis 0.0) 0.0 1.0) (* (Utilities|Time|GetWorldDeltaSeconds) (Variables|Speed|GetMoveSpeed))) (Math|Vector|Normalize (Math|Vector|MakeVector 0.0 (.Y (Math|Vector|BreakVector (.Normal (Collision|BreakHitResult _sweephitresult)))) 0.0))) (- 1.0 (.Time (Collision|BreakHitResult _sweephitresult)))) true))))

(event Custom|InmputFireForvard_For_Server
  (params (NewParam :type Float%20%28single-precision%29))
  ;[1 1 1] Стрельба
  (CallFunction|InmputFireForvardforAll NewParam))

(event Custom|InmputFireForvard_For_All
  (params (NewParam :type Float%20%28single-precision%29))
  ;[1 1 1] Стрельба
  (if (Variables|Default|GetEnergy_Fire_Activate?)
    (CallFunction|FireLeftMousEnergy (Math|Vector|MakeVector NewParam (stale Custom|InmputFireRight_For_All NewParam) 0.0))
    (else
      (CallFunction|FireLeftMousKinetic (Math|Vector|MakeVector NewParam (stale Custom|InmputFireRight_For_All NewParam) 0.0) (Utilities|Array|Get(acopy) (Variables|KineticWeapon|GetKinetic_Spread_Var) (Variables|KineticWeapon|GetKinetik_Spread_index)))
      (if (< (Variables|KineticWeapon|GetKinetik_Spread_index) 19)
        (Math|Integer|IncrementInt (Variables|KineticWeapon|GetKinetik_Spread_index))
        (else
          (Variables|KineticWeapon|SetKinetik_Spread_index 0))))))

(event EventPossessed
  (params (NewController :type Controller%20Object%20Reference))
  ;[1 1 1] Записать владельца
  (CallFunction|EventonPossesedCallServer))

(event EventBeginPlay
  ;[1 1 1] Регенерация статов
  (CallFunction|RefreshEnergy)
  (CallFunction|RefreshShield)
  (CallFunction|RefreshHP))

(event Game|Damage|EventAnyDamage
  (params (Damage :type Float%20%28single-precision%29) (DamageType :type Damage%20Type%20Object%20Reference) (InstigatedBy :type Controller%20Object%20Reference) (DamageCauser :type Actor%20Object%20Reference))
  ;[1 1 1] Получение урона и смерть
  (switch Utilities|FlowControl|Switch|SwitchonDamage_Type_E_Num (Variables|/Game/PlayerCharacter/Blueprints/Projectiles/Parrent_Projectile.Parrent_Projectile_C|GetDamage_type (.AsParrent%20Projectile (Utilities|Casting|CastToParrent_Projectile DamageCauser)))
    (:NewEnumerator0
      (if (> (Variables|Ship_Stats|GetCurrent_Armor) 0.0)
        (Variables|Ship_Stats|SetCurrent_Armor (- (Variables|Ship_Stats|GetCurrent_Armor) (|(Damage*koeffArmor) Damage (Variables|Damage_Math|GetKinetic_Damage_To_Armor_Koeff))))
        (Variables|Ship_Stats|SetCurrent_HP (- (Variables|Ship_Stats|GetCurrent_HP) (|(Damage*Koeff_HP) Damage (Variables|Damage_Math|GetKinetic_Damage_To_HP_Koeff))))
        (else
          (Variables|Ship_Stats|SetCurrent_HP (- (Variables|Ship_Stats|GetCurrent_HP) Damage))))
      (Development|PrintString (Utilities|String|ToString(Float) (Variables|Ship_Stats|GetCurrent_HP)))
      (Development|PrintString (Utilities|String|ToString(Float) (Variables|Ship_Stats|GetCurrent_Armor))))
    (:NewEnumerator1
      (if (> (Variables|Ship_Stats|GetCurrent_Armor) 0.0)
        (Variables|Ship_Stats|SetCurrent_Armor (- (Variables|Ship_Stats|GetCurrent_Armor) (|(Damage*koeff_Armor) Damage (Variables|Damage_Math|GetEnergy_Damage_To_Armor_Koeff))))
        (Variables|Ship_Stats|SetCurrent_HP (- (Variables|Ship_Stats|GetCurrent_HP) (|(Damage*Koeff_HP) Damage (Variables|Damage_Math|GetEnergy_Damage_To_HP_Koeff))))
        (else
          (Variables|Ship_Stats|SetCurrent_HP (- (Variables|Ship_Stats|GetCurrent_HP) (|(Damage*Koeff_Pure_HP) Damage (Variables|Damage_Math|GetEnergy_Damage_TO_HP_Pure))))))
      (Development|PrintString (Utilities|String|ToString(Float) (Variables|Ship_Stats|GetCurrent_HP)))
      (Development|PrintString (Utilities|String|ToString(Float) (Variables|Ship_Stats|GetCurrent_Armor))))
    (:NewEnumerator2
      (Variables|Ship_Stats|SetCurrent_HP (- (Variables|Ship_Stats|GetCurrent_HP) Damage))
      (Variables|Ship_Stats|SetCurrent_Armor (- (Variables|Ship_Stats|GetCurrent_Armor) Damage))
      (Development|PrintString (Utilities|String|ToString(Float) (Variables|Ship_Stats|GetCurrent_HP)))
      (Development|PrintString (Utilities|String|ToString(Float) (Variables|Ship_Stats|GetCurrent_Armor))))
    (:NewEnumerator3
      (Variables|Ship_Stats|SetCurrent_HP (- (Variables|Ship_Stats|GetCurrent_HP) Damage))
      (Development|PrintString (Utilities|String|ToString(Float) (Variables|Ship_Stats|GetCurrent_HP)))))
  (if (Variables|Default|GetBattle_Mode_Activate?)
    _
    (else
      (CallFunction|TakeDamageinTravelMode)))
  (if (<= (Variables|Ship_Stats|GetCurrent_HP) 0.0)
    (Utilities|FlowControl|DoOnce false
      (:Completed
        (CallFunction|DeathCallAll)))))

(event Input|ActionEvents|InputActionSwitch_Fire_Type
  (params (Key :type Key%20Structure :default "None"))
  ;[1 1 1] Активация енергитических выстрелов
  (:Pressed
    (if (Variables|Default|GetBattle_Mode_Activate?)
      (CallFunction|SwitchFireTypeCallServer))))

(event Input|ActionEvents|InputActionSwap_Battle_mode
  (params (Key :type Key%20Structure :default "None"))
  ;[1 1 1] Смена тревел/батл мода
  (:Pressed
    (CallFunction|SwapBattleModeCallServer)))

(event Input|ActionEvents|InputActionFire_Rockets
  (params (Key :type Key%20Structure :default "None"))
  ;[1 1 1] Rocket
  (:Pressed
    (if (Variables|Default|GetBattle_Mode_Activate?)
      (CallFunction|FireRocketforServer))))

(event Input|AxisEvents|InputAxisMoveForward
  (params (AxisValue :type Float%20%28single-precision%29))
  ;[1 1 1] Передвижение
  (CallFunction|MoveForwardCallServer AxisValue))

(event Input|AxisEvents|InputAxisMoveRight
  (params (AxisValue :type Float%20%28single-precision%29))
  ;[1 1 1] Передвижение
  (CallFunction|MuveRightCallServer AxisValue))

(event Input|AxisEvents|InputAxisFire_Forvard
  (params (AxisValue :type Float%20%28single-precision%29))
  ;[1 1 1] Стрельба
  (if (Variables|Default|GetBattle_Mode_Activate?)
    (CallFunction|InmputFireForvardforServer AxisValue)))

(event Input|AxisEvents|InputAxisFire_Right
  (params (AxisValue :type Float%20%28single-precision%29))
  ;[1 1 1] Стрельба
  (if (Variables|Default|GetBattle_Mode_Activate?)
    (CallFunction|InmputFireRightforServer AxisValue)))

(event Input|KeyboardEvents|T
  (params (Key :type Key%20Structure :default "None"))
  (:Pressed
    (Development|PrintString "Hello" true true "(R=1.000000,G=0.000000,B=0.033492,A=1.000000)")))

(fn ConstructionScript)

(fn FireLeftMousKinetic
  (params (direction :type Vector) (Spread_Weapon :type Float%20%28single-precision%29))
  (bind _returnvalue (Math|Conversions|RotationFromXVector direction))
  (if (Variables|Default|GetCanFire)
    (if (> (Math|Vector|VectorLength direction) 0.0)
      (bind _returnvalue_2 (Game|SpawnActorfromClass "/Game/PlayerCharacter/Blueprints/Projectiles/Childe_Kinetic_Projectile.Childe_Kinetic_Projectile_C" (Math|Transform|MakeTransform (+ (Transformation|GetActorLocation) (Math|Vector|RotateVector (Variables|Kinetic_Weapon|GetGunOffset_kinetic) _returnvalue)) (Math|Rotator|MakeRotator 0.0 0.0 (+ (.yaw (.rotation (Math|Transform|MakeTransform "0, 0, 0" _returnvalue))) Spread_Weapon)) "1,1,1") "AlwaysSpawn" 0 self))
      (Variables|/Game/PlayerCharacter/Blueprints/Projectiles/Childe_Kinetic_Projectile.Childe_Kinetic_Projectile_C|SetKinetic_Projectile_Damage _returnvalue_2 (Variables|Kinetic_Weapon|GetKinetic_Damage))
      (Variables|/Game/PlayerCharacter/Blueprints/Projectiles/Childe_Kinetic_Projectile.Childe_Kinetic_Projectile_C|SetOwner_REF _returnvalue_2 self)
      (Variables|/Game/PlayerCharacter/Blueprints/Projectiles/Childe_Kinetic_Projectile.Childe_Kinetic_Projectile_C|Setteam_Projectile_Number _returnvalue_2 (Variables|Default|GetCharacter_Number))
      (Variables|Default|SetCanFire false)
      (Utilities|Time|SetTimerbyFunctionName 0 "Shoot_Kinetic_Timer_Expired" (Variables|Kinetic_Weapon|GetAttack_Speed_kinetic)))))

(fn ShootEnergyTimerExpired
  (Variables|Default|SetCanFire true))

(fn ShootKineticTimerExpired
  (Variables|Default|SetCanFire true))

(fn FireLeftMousEnergy
  (params (Direction :type Vector))
  (bind _returnvalue (Math|Conversions|RotationFromXVector Direction))
  (if (Variables|Default|GetCanFire)
    (if (> (Math|Vector|VectorLength Direction) 0.0)
      (if (>= (Variables|Ship_Stats|GetCurrent_Energy) (Variables|Energy_Weapon|GetEnergy_Weapon_Cost))
        (bind _output_get (Variables|Ship_Stats|SetCurrent_Energy (- (Variables|Ship_Stats|GetCurrent_Energy) (Variables|Energy_Weapon|GetEnergy_Weapon_Cost))))
        (Development|PrintString (Utilities|String|ToString(Float) _output_get))
        (bind _returnvalue_2 (Game|SpawnActorfromClass "/Game/PlayerCharacter/Blueprints/Projectiles/Childe_Energy_Projectile.Childe_Energy_Projectile_C" (Math|Transform|MakeTransform (+ (Transformation|GetActorLocation) (Math|Vector|RotateVector (Variables|Energy_Weapon|GetGunOffset_Energy) _returnvalue)) _returnvalue "1,1,1") "AlwaysSpawn" 0 self))
        (Variables|/Game/PlayerCharacter/Blueprints/Projectiles/Childe_Energy_Projectile.Childe_Energy_Projectile_C|SetEnergy_Projectile_Damage _returnvalue_2 (Variables|Energy_Weapon|GetEnergy_Damage))
        (Variables|/Game/PlayerCharacter/Blueprints/Projectiles/Childe_Energy_Projectile.Childe_Energy_Projectile_C|SetOwner_REF _returnvalue_2 self)
        (Variables|/Game/PlayerCharacter/Blueprints/Projectiles/Childe_Energy_Projectile.Childe_Energy_Projectile_C|Setteam_Projectile_Number _returnvalue_2 (Variables|Default|GetCharacter_Number))
        (Variables|Default|SetCanFire false)
        (Utilities|Time|SetTimerbyFunctionName 0 "Shoot_Energy_Timer_Expired" (Variables|Energy_Weapon|GetAttack_Speed_Energy))
        (else
          (CallFunction|AutoSwitchFireType))))))

(fn ShootRocket
  (if (> (Variables|Rocket_Weapon|GetCurrent_Value_Rockets) 0)
    (Variables|Rocket_Weapon|SetCurrent_Value_Rockets (- (Variables|Rocket_Weapon|GetCurrent_Value_Rockets) 1))
    (bind _returnvalue (Game|SpawnActorfromClass "/Game/PlayerCharacter/Blueprints/Projectiles/Childe_Rocket_Projectile.Childe_Rocket_Projectile_C" (Math|Transform|MakeTransform (+ (Transformation|GetActorLocation) (Variables|RocketWeapon|GetGunOffset_Rocket)) (Transformation|GetActorRotation) "1,1,1") "AlwaysSpawn" 0 0))
    (Variables|/Game/PlayerCharacter/Blueprints/Projectiles/Childe_Rocket_Projectile.Childe_Rocket_Projectile_C|SetRocket_Projectile_Damage _returnvalue (Variables|Rocket_Weapon|GetRocket_Damage))
    (Variables|/Game/PlayerCharacter/Blueprints/Projectiles/Childe_Rocket_Projectile.Childe_Rocket_Projectile_C|SetTeam_Projectile_Number _returnvalue (Variables|Default|GetCharacter_Number))))