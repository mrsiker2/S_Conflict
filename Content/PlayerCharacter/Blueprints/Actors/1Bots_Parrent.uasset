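; Base class for team combat bots that detect enemies, shoot and take damage.
; AI perception feeds a Server-to-All event chain that acquires an enemy bot or character, fires empty start-fire hooks, and rescans for the nearest enemy when the current target updates.
; Shared functions spawn aimed kinetic, energy, snipe and rocket projectiles with team and level-based damage.
; AnyDamage splits damage between armor and HP by projectile type, destroying the bot at zero HP.
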(event OnTargetPerceptionUpdated(AIPerception)
  (params (Actor :type Actor%20Object%20Reference) (Stimulus :type AI%20Stimulus%20Structure))
  ;[1 1 1] Так выглядит стрельба
  (CallFunction|CheckEnemyCallServer Actor))

(event OnPerceptionUpdated(AIPerception)
  (params (UpdatedActors :type Array%20of%20Actor%20Object%20References))
  ;[1 1 1] Так выглядит стрельба
)

(event Custom|Bot_Death_Call_All
  ;[1 1 1] Получение урона
  (Actor|DestroyActor))

(event Custom|Energy_Start_Fire_Bot
  ;[1 1 1] Так выглядит стрельба
)

(event Custom|Snipe_Energy_Start_Fire_Bot
  ;[1 1 1] Так выглядит стрельба
)

(event Custom|Rocket_Start_Fire_Bot
  ;[1 1 1] Так выглядит стрельба
)

(event Custom|Check_Enemy_Call_Server
  (params (actor1 :type Actor%20Object%20Reference))
  ;[1 1 1] Так выглядит стрельба
  (CallFunction|CheckEnemyCallAll actor1))

(event Custom|Check_Enemy_Call_All
  (params (actor1 :type Actor%20Object%20Reference))
  ;[1 1 1] Так выглядит стрельба
  (Utilities|FlowControl|Delay 0.01)
  (if (== actor1 (Variables|Default|GetTarget_For_Fire))
    (Variables|Default|SetTarget_For_Fire_REF (Variables|Default|GetTarget_For_Fire))
    (Variables|Default|SetEnemy_In_Radius? false)
    (Variables|Default|SetMinimal_Distance_For_Focus 2e+03)
    (Variables|Default|SetVAR_FOR_CHECK_ENEMY 0)
    (for _array_element (stale OnPerceptionUpdated(AIPerception) UpdatedActors)
      (bind _as1bots_parrent (Utilities|Casting|CastTo1Bots_Parrent _array_element)
        (:then
          (if (not (== (Variables|1Bots_Parrent_C|GetBot_Team_Number _as1bots_parrent) (Variables|Default|GetBot_Team_Number)))
            (if (>= (Variables|Default|GetMinimal_Distance_For_Focus) (Transformation|GetDistanceTo _as1bots_parrent))
              (Variables|Default|SetMinimal_Distance_For_Focus (Transformation|GetDistanceTo _as1bots_parrent))
              (Variables|Default|SetTarget_For_Fire _as1bots_parrent)
              (Variables|Default|SetEnemy_In_Radius? true)
              (Math|Integer|IncrementInt (Variables|Default|GetVAR_FOR_CHECK_ENEMY)))))
        (:CastFailed
          (bind _asmain_character (Utilities|Casting|CastToMain_Character _array_element))
          (if (not (== (Variables|/Game/PlayerCharacter/Blueprints/Main_Char/Main_Character.Main_Character_C|GetCharacter_Number _asmain_character) (Variables|Default|GetBot_Team_Number)))
            (if (>= (Variables|Default|GetMinimal_Distance_For_Focus) (Transformation|GetDistanceTo _asmain_character))
              (if (== (Variables|Default|GetTarget_For_Fire_REF) (Variables|Default|GetTarget_For_Fire))
                (Variables|Default|SetTarget_For_Fire (Variables|Default|GetTarget_for_Fire_NONE))
                (Variables|Default|SetEnemy_In_Radius? false)
                (else
                  (Variables|Default|SetMinimal_Distance_For_Focus (Transformation|GetDistanceTo _asmain_character))
                  (Variables|Default|SetTarget_For_Fire _asmain_character)
                  (Variables|Default|SetEnemy_In_Radius? true)
                  (Math|Integer|IncrementInt (Variables|Default|GetVAR_FOR_CHECK_ENEMY)))))))))
    (if (== (Variables|Default|GetVAR_FOR_CHECK_ENEMY) 0)
      (Variables|Default|SetTarget_For_Fire (Variables|Default|GetTarget_for_Fire_NONE))
      (Variables|Default|SetEnemy_In_Radius? false))
    (else
      (Utilities|IsValid (Variables|Default|GetTarget_For_Fire)
        (:Is%20Not%20Valid
          (bind _as1bots_parrent_2 (Utilities|Casting|CastTo1Bots_Parrent actor1)
            (:then
              (if (not (== (Variables|1Bots_Parrent_C|GetBot_Team_Number _as1bots_parrent_2) (Variables|Default|GetBot_Team_Number)))
                (Variables|Default|SetEnemy_In_Radius? true)
                (Variables|Default|SetTarget_For_Fire _as1bots_parrent_2)
                (CallFunction|KineticStartFireBot)
                (CallFunction|SnipeEnergyStartFireBot)
                (CallFunction|RocketStartFireBot)
                (CallFunction|EnergyStartFireBot)))
            (:CastFailed
              (bind _asmain_character_2 (Utilities|Casting|CastToMain_Character actor1))
              (if (not (== (Variables|/Game/PlayerCharacter/Blueprints/Main_Char/Main_Character.Main_Character_C|GetCharacter_Number _asmain_character_2) (Variables|Default|GetBot_Team_Number)))
                (Variables|Default|SetEnemy_In_Radius? true)
                (Variables|Default|SetTarget_For_Fire _asmain_character_2)
                (CallFunction|KineticStartFireBot)
                (CallFunction|SnipeEnergyStartFireBot)
                (CallFunction|RocketStartFireBot)
                (CallFunction|EnergyStartFireBot)))))))))

(event Custom|Kinetic_Start_Fire_Bot
  ;[1 1 1] Так выглядит стрельба
)

(event Game|Damage|EventAnyDamage
  (params (Damage :type Float%20%28single-precision%29) (DamageType :type Damage%20Type%20Object%20Reference) (InstigatedBy :type Controller%20Object%20Reference) (DamageCauser :type Actor%20Object%20Reference))
  ;[1 1 1] Получение урона
  (switch Utilities|FlowControl|Switch|SwitchonDamage_Type_E_Num (Variables|/Game/PlayerCharacter/Blueprints/Projectiles/Parrent_Projectile.Parrent_Projectile_C|GetDamage_type (.AsParrent%20Projectile (Utilities|Casting|CastToParrent_Projectile DamageCauser)))
    (:NewEnumerator0
      (if (> (Variables|Object_Health|GetCurrent_Armor) 0.0)
        (Variables|Object_Health|SetCurrent_Armor (- (Variables|Object_Health|GetCurrent_Armor) (|(Damage*koeffArmor) Damage (Variables|Math_Koeff|GetKinetic_Damage_To_Armor_Koeff))))
        (Variables|Object_Health|SetCurrent_HP (- (Variables|Object_Health|GetCurrent_HP) (|(Damage*Koeff_HP) Damage (Variables|Math_Koeff|GetKinetic_Damage_To_HP_Koeff))))
        (else
          (Variables|Object_Health|SetCurrent_HP (- (Variables|Object_Health|GetCurrent_HP) Damage))))
      (Development|PrintString (Utilities|String|ToString(Float) (Variables|Object_Health|GetCurrent_HP)))
      (Development|PrintString (Utilities|String|ToString(Float) (Variables|Object_Health|GetCurrent_Armor))))
    (:NewEnumerator1
      (if (> (Variables|Object_Health|GetCurrent_Armor) 0.0)
        (Variables|Object_Health|SetCurrent_Armor (- (Variables|Object_Health|GetCurrent_Armor) (|(Damage*koeff_Armor) Damage (Variables|Math_Koeff|GetEnergy_Damage_To_Armor_Koeff))))
        (Variables|Object_Health|SetCurrent_HP (- (Variables|Object_Health|GetCurrent_HP) (|(Damage*Koeff_HP) Damage (Variables|Math_Koeff|GetEnergy_Damage_To_HP_Koeff))))
        (else
          (Variables|Object_Health|SetCurrent_HP (- (Variables|Object_Health|GetCurrent_HP) (|(Damage*Koeff_Pure_HP) Damage (Variables|Math_Koeff|GetEnergy_Damage_To_HP_Pure))))))
      (Development|PrintString (Utilities|String|ToString(Float) (Variables|Object_Health|GetCurrent_HP)))
      (Development|PrintString (Utilities|String|ToString(Float) (Variables|Object_Health|GetCurrent_Armor))))
    (:NewEnumerator2
      (Variables|Object_Health|SetCurrent_HP (- (Variables|Object_Health|GetCurrent_HP) Damage))
      (Variables|Object_Health|SetCurrent_Armor (- (Variables|Object_Health|GetCurrent_Armor) Damage))
      (Development|PrintString (Utilities|String|ToString(Float) (Variables|Object_Health|GetCurrent_HP)))
      (Development|PrintString (Utilities|String|ToString(Float) (Variables|Object_Health|GetCurrent_Armor))))
    (:NewEnumerator3
      (Variables|Object_Health|SetCurrent_HP (- (Variables|Object_Health|GetCurrent_HP) Damage))
      (Development|PrintString (Utilities|String|ToString(Float) (Variables|Object_Health|GetCurrent_HP)))
      (Development|PrintString (Utilities|String|ToString(Float) (Variables|Object_Health|GetCurrent_Armor)))))
  (if (<= (Variables|Object_Health|GetCurrent_HP) 0.0)
    (Utilities|FlowControl|DoOnce false
      (:Completed
        (CallFunction|BotDeathCallAll)))))

(fn ConstructionScript)

(fn KineticFireWeapon
  (params (Gun_Location :type Vector) (Gun_Offsett :type Vector) (Target_For_fire :type Actor%20Object%20Reference) (Spread_Weapon :type Float%20%28single-precision%29))
  (bind _returnvalue (Transformation|GetActorLocation Target_For_fire))
  (bind _returnvalue_2 (Math|Rotator|FindLookatRotation Gun_Location _returnvalue))
  (bind _returnvalue_3 (Game|SpawnActorfromClass "/Game/PlayerCharacter/Blueprints/Projectiles/Childe_Kinetic_Projectile.Childe_Kinetic_Projectile_C" (Math|Transform|MakeTransform (+ Gun_Location (Math|Vector|RotateVector Gun_Offsett (Math|Rotator|MakeRotator (.roll _returnvalue_2) (.pitch _returnvalue_2) (.yaw _returnvalue_2)))) (Math|Rotator|MakeRotator 0.0 0.0 (+ (.yaw _returnvalue_2) (Math|Random|RandomFloatinRange (* -1 Spread_Weapon) Spread_Weapon))) "1,1,1") "AlwaysSpawn" 0 self))
  (switch Utilities|FlowControl|Switch|SwitchonKINETIC_LVL_DMG (Variables|E_NUM_Variable_LVL|GetKinetic_DMG_LVL)
    (:NewEnumerator0
      (Variables|/Game/PlayerCharacter/Blueprints/Projectiles/Childe_Kinetic_Projectile.Childe_Kinetic_Projectile_C|SetKinetic_Projectile_Damage _returnvalue_3 (Variables|Kinetic_Weapon_Stats|GetKinetic_LVL_1_DMG)))
    (:NewEnumerator1
      (Variables|/Game/PlayerCharacter/Blueprints/Projectiles/Childe_Kinetic_Projectile.Childe_Kinetic_Projectile_C|SetKinetic_Projectile_Damage _returnvalue_3 (Variables|Kinetic_Weapon_Stats|GetKinetic_LVL_2_DMG)))
    (:NewEnumerator2
      (Variables|/Game/PlayerCharacter/Blueprints/Projectiles/Childe_Kinetic_Projectile.Childe_Kinetic_Projectile_C|SetKinetic_Projectile_Damage _returnvalue_3 (Variables|Kinetic_Weapon_Stats|GetKinetic_LVL_3_DMG))))
  (Variables|/Game/PlayerCharacter/Blueprints/Projectiles/Childe_Kinetic_Projectile.Childe_Kinetic_Projectile_C|Setteam_Projectile_Number _returnvalue_3 (Variables|Default|GetBot_Team_Number))
  (Variables|/Script/Engine.ProjectileMovementComponent|SetMaxSpeed (Variables|/Game/PlayerCharacter/Blueprints/Projectiles/Childe_Kinetic_Projectile.Childe_Kinetic_Projectile_C|GetProjectileMovement _returnvalue_3) (Variables|Kinetic_Weapon_Stats|GetKinetic_Projectile_Speed))
  (Variables|/Script/Engine.ProjectileMovementComponent|SetInitialSpeed (Variables|/Game/PlayerCharacter/Blueprints/Projectiles/Childe_Kinetic_Projectile.Childe_Kinetic_Projectile_C|GetProjectileMovement _returnvalue_3) (Variables|Kinetic_Weapon_Stats|GetKinetic_Projectile_Speed)))

(fn EnergyFireWeapon
  (params (Gun_Location :type Vector) (Gun_Offsett :type Vector) (Target_for_Fire :type Actor%20Object%20Reference) (Spread_Weapon :type Float%20%28single-precision%29))
  (bind _returnvalue (Transformation|GetActorLocation Target_for_Fire))
  (bind _returnvalue_2 (Math|Rotator|FindLookatRotation Gun_Location _returnvalue))
  (bind _returnvalue_3 (Game|SpawnActorfromClass "/Game/PlayerCharacter/Blueprints/Projectiles/Childe_Energy_Projectile.Childe_Energy_Projectile_C" (Math|Transform|MakeTransform (+ Gun_Location (Math|Vector|RotateVector Gun_Offsett (Math|Rotator|MakeRotator (.roll _returnvalue_2) (.pitch _returnvalue_2) (.yaw _returnvalue_2)))) (Math|Rotator|MakeRotator 0.0 0.0 (+ (.yaw _returnvalue_2) (Math|Random|RandomFloatinRange (* -1 Spread_Weapon) Spread_Weapon))) "1,1,1") "AlwaysSpawn" 0 self))
  (switch Utilities|FlowControl|Switch|SwitchonENERGY_LVL_DMG (Variables|ENUMVariableLVL|GetEnergy_DMG_LVL)
    (:NewEnumerator0
      (Variables|/Game/PlayerCharacter/Blueprints/Projectiles/Childe_Energy_Projectile.Childe_Energy_Projectile_C|SetEnergy_Projectile_Damage _returnvalue_3 (Variables|Energy_Weapon_Stats|GetEnergy_LVL_1_DMG)))
    (:NewEnumerator1
      (Variables|/Game/PlayerCharacter/Blueprints/Projectiles/Childe_Energy_Projectile.Childe_Energy_Projectile_C|SetEnergy_Projectile_Damage _returnvalue_3 (Variables|Energy_Weapon_Stats|GetEnergy_LVL_2_DMG)))
    (:NewEnumerator2
      (Variables|/Game/PlayerCharacter/Blueprints/Projectiles/Childe_Energy_Projectile.Childe_Energy_Projectile_C|SetEnergy_Projectile_Damage _returnvalue_3 (Variables|Energy_Weapon_Stats|GetEnergy_LVL_3_DMG))))
  (Variables|/Game/PlayerCharacter/Blueprints/Projectiles/Childe_Energy_Projectile.Childe_Energy_Projectile_C|Setteam_Projectile_Number _returnvalue_3 (Variables|Default|GetBot_Team_Number))
  (Variables|/Script/Engine.ProjectileMovementComponent|SetMaxSpeed (Variables|/Game/PlayerCharacter/Blueprints/Projectiles/Childe_Energy_Projectile.Childe_Energy_Projectile_C|GetProjectileMovement _returnvalue_3) (Variables|Energy_Weapon_Stats|GetEnergy_Projectile_Speed))
  (Variables|/Script/Engine.ProjectileMovementComponent|SetInitialSpeed (Variables|/Game/PlayerCharacter/Blueprints/Projectiles/Childe_Energy_Projectile.Childe_Energy_Projectile_C|GetProjectileMovement _returnvalue_3) (Variables|Energy_Weapon_Stats|GetEnergy_Projectile_Speed)))

(fn EnergyFireSnipeShot
  (params (Gun_Location :type Vector) (Gun_Offsett :type Vector) (Target_For_Fire :type Actor%20Object%20Reference))
  (bind _returnvalue (Transformation|GetActorLocation Target_For_Fire))
  (bind _returnvalue_2 (Math|Rotator|FindLookatRotation Gun_Location _returnvalue))
  (bind _returnvalue_3 (Game|SpawnActorfromClass "/Game/PlayerCharacter/Blueprints/Projectiles/Childe_Energy_Projectile_SNIPE_SHOT.Childe_Energy_Projectile_SNIPE_SHOT_C" (Math|Transform|MakeTransform (+ Gun_Location (Math|Vector|RotateVector Gun_Offsett (Math|Rotator|MakeRotator (.roll _returnvalue_2) (.pitch _returnvalue_2) (.yaw _returnvalue_2)))) (Math|Rotator|MakeRotator 0.0 0.0 (.yaw _returnvalue_2)) "1,1,1") "AlwaysSpawn" 0 self))
  (switch Utilities|FlowControl|Switch|SwitchonENERGY_SNYPE_SHOT_LVL_DMG (Variables|ENUMVariableLVL|GetEnergy_Snipe_Shot_DMG_LVL)
    (:NewEnumerator0
      (Variables|/Game/PlayerCharacter/Blueprints/Projectiles/Childe_Energy_Projectile.Childe_Energy_Projectile_C|SetEnergy_Projectile_Damage _returnvalue_3 (Variables|Energy_Snype_Weapon|GetSnipe_Energy_LVL_1_DMG)))
    (:NewEnumerator1
      (Variables|/Game/PlayerCharacter/Blueprints/Projectiles/Childe_Energy_Projectile.Childe_Energy_Projectile_C|SetEnergy_Projectile_Damage _returnvalue_3 (Variables|Energy_Snype_Weapon|GetSnipe_Energy_LVL_2_DMG)))
    (:NewEnumerator2
      (Variables|/Game/PlayerCharacter/Blueprints/Projectiles/Childe_Energy_Projectile.Childe_Energy_Projectile_C|SetEnergy_Projectile_Damage _returnvalue_3 (Variables|Energy_Snype_Weapon|GetSnipe_Energy_LVL_3_DMG))))
  (Variables|/Game/PlayerCharacter/Blueprints/Projectiles/Childe_Energy_Projectile.Childe_Energy_Projectile_C|Setteam_Projectile_Number _returnvalue_3 (Variables|Default|GetBot_Team_Number))
  (Variables|/Game/PlayerCharacter/Blueprints/Projectiles/Childe_Energy_Projectile_SNIPE_SHOT.Childe_Energy_Projectile_SNIPE_SHOT_C|SetTarget_For_Snipe_Shot _returnvalue_3 Target_For_Fire)
  (Variables|/Game/PlayerCharacter/Blueprints/Projectiles/Childe_Energy_Projectile_SNIPE_SHOT.Childe_Energy_Projectile_SNIPE_SHOT_C|SetSnipe_Shot_Projectile_Interp_Speed _returnvalue_3 (Variables|Energy_Snype_Weapon|GetSnipe_Energy_Projectile_Speed)))

(fn RocketFireWeapon
  (params (Gun_Location :type Vector) (Gun_Offset :type Vector) (Target_For_Fire :type Actor%20Object%20Reference))
  (bind _returnvalue (Transformation|GetActorLocation Target_For_Fire))
  (bind _returnvalue_2 (Math|Rotator|FindLookatRotation Gun_Location _returnvalue))
  (bind _returnvalue_3 (Game|SpawnActorfromClass "/Game/PlayerCharacter/Blueprints/Projectiles/Childe_Rocket_Projectile.Childe_Rocket_Projectile_C" (Math|Transform|MakeTransform (+ Gun_Location (Math|Vector|RotateVector Gun_Offset (Math|Rotator|MakeRotator (.roll _returnvalue_2) (.pitch _returnvalue_2) (.yaw _returnvalue_2)))) (Math|Rotator|MakeRotator 0.0 0.0 (.yaw _returnvalue_2)) "1,1,1") "AlwaysSpawn" 0 self))
  (switch Utilities|FlowControl|Switch|SwitchonROCKET_LVL_DMG (Variables|ENUMVariableLVL|GetRocket_DMG_LVL)
    (:NewEnumerator0
      (Variables|/Game/PlayerCharacter/Blueprints/Projectiles/Childe_Rocket_Projectile.Childe_Rocket_Projectile_C|SetRocket_Projectile_Damage _returnvalue_3 (Variables|Rocket_Weapon_Stats|GetRocket_LVL_1_DMG)))
    (:NewEnumerator1
      (Variables|/Game/PlayerCharacter/Blueprints/Projectiles/Childe_Rocket_Projectile.Childe_Rocket_Projectile_C|SetRocket_Projectile_Damage _returnvalue_3 (Variables|Rocket_Weapon_Stats|GetRocket_LVL_2_DMG)))
    (:NewEnumerator2
      (Variables|/Game/PlayerCharacter/Blueprints/Projectiles/Childe_Rocket_Projectile.Childe_Rocket_Projectile_C|SetRocket_Projectile_Damage _returnvalue_3 (Variables|Rocket_Weapon_Stats|GetRocket_LVL_3_DMG))))
  (Variables|/Game/PlayerCharacter/Blueprints/Projectiles/Childe_Rocket_Projectile.Childe_Rocket_Projectile_C|SetTeam_Projectile_Number _returnvalue_3 (Variables|Default|GetBot_Team_Number)))