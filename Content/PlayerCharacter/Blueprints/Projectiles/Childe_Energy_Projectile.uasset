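; Child energy projectile Blueprint that damages bots or player characters of a different team on overlap.
; Overlap casts the other actor to the bot parent or main character class and compares its team number against the projectile's.
; On a mismatch it hides the mesh, waits briefly, then applies point damage once through a DoOnce and destroys itself.
; Only the player-character branch passes an event instigator.
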(event `self.StaticMesh.OnComponentBeginOverlap`
  (params (OverlappedComponent :type "PrimitiveComponent Object Reference") (OtherActor :type "Actor Object Reference") (OtherComp :type "PrimitiveComponent Object Reference") (OtherBodyIndex :type Integer) (bFromSweep :type Boolean) (SweepResult :type "HitResult Structure (by ref)"))
  (bind (_bblockinghit _binitialoverlap _time _distance _location _impactpoint _normal _impactnormal _physmat _hitactor _hitcomponent _hitbonename _hititem _elementindex _faceindex _tracestart _traceend) (`GameplayStatics.BreakHitResult` SweepResult))
  (bind (_bblockinghit_2 _binitialoverlap_2 _time_2 _distance_2 _location_2 _impactpoint_2 _normal_2 _impactnormal_2 _physmat_2 _hitactor_2 _hitcomponent_2 _hitbonename_2 _hititem_2 _elementindex_2 _faceindex_2 _tracestart_2 _traceend_2) (`GameplayStatics.BreakHitResult` SweepResult))
  (`KismetSystemLibrary.Delay` 0.001)
  (bind _asbots_parrent (cast `/Game/PlayerCharacter/Blueprints/Actors/1Bots_Parrent` OtherActor)
    (:`then`
      (if (!= (`self.team_Projectile_Number`) (`/Game/PlayerCharacter/Blueprints/Actors/1Bots_Parrent.Bot_Team_Number` _asbots_parrent))
        (`SceneComponent.SetHiddenInGame` (`self.StaticMesh`) true true)
        (`KismetSystemLibrary.Delay` 0.002)
        (`/Engine/EditorBlueprintResources/StandardMacros.DoOnce` false
          (:`Completed`
            (`GameplayStatics.ApplyPointDamage` _asbots_parrent (`self.Energy_Projectile_Damage`) (`KismetMathLibrary.GetDirectionUnitVector` _traceend_2 _tracestart_2) SweepResult null self)
            (`self.K2_DestroyActor`)))))
    (:`CastFailed`
      (bind _asmain_character (cast `/Game/PlayerCharacter/Blueprints/Main_Char/Main_Character` OtherActor))
      (if (!= (`self.team_Projectile_Number`) (`/Game/PlayerCharacter/Blueprints/Main_Char/Main_Character.Character_Number` _asmain_character))
        (`SceneComponent.SetHiddenInGame` (`self.StaticMesh`) true true)
        (`KismetSystemLibrary.Delay` 0.002)
        (`/Engine/EditorBlueprintResources/StandardMacros.DoOnce` false
          (:`Completed`
            (`GameplayStatics.ApplyPointDamage` OtherActor (`self.Energy_Projectile_Damage`) (`KismetMathLibrary.GetDirectionUnitVector` _traceend _tracestart) SweepResult (`self.GetInstigatorController`) self)
            (`self.K2_DestroyActor`)))))))

(fn `UserConstructionScript`
  (`parent.UserConstructionScript`))