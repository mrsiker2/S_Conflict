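; Child rocket projectile that homes in on an enemy bot or player character and deals point damage.
; Shortly after spawn, one forward box trace picks the nearest pawn from another team.
; Tick moves the rocket along its mesh's forward vector and, through a gate opened once a target exists, turns the mesh toward it at constant speed.
; Overlapping an opposing pawn hides the mesh, applies damage once and destroys the rocket.
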(event `self.ReceiveBeginPlay`
  (bind _staticmesh (`self.StaticMesh`))
  (bind _returnvalue (`SceneComponent.K2_GetComponentLocation` _staticmesh))
  ;[1 1 1] Было 0.5
  (`KismetSystemLibrary.Delay` 0.2)
  (bind _outhits (`KismetSystemLibrary.BoxTraceMultiForObjects` :`Start` _returnvalue :`End` (+ _returnvalue (* (`SceneComponent.GetForwardVector` _staticmesh) 2500.0)) :`HalfSize` (300.0 300.0 20.0) :`ObjectTypes` (`|MakeArray` "ObjectTypeQuery3" :!type "EObjectTypeQuery Enum") :`DrawDebugType` "ForDuration"))
  (for _array_element _outhits
    (bind (_bblockinghit _binitialoverlap _time _distance _location _impactpoint _normal _impactnormal _physmat _hitactor) (`GameplayStatics.BreakHitResult` _array_element))
    (bind _asbots_parrent (cast `/Game/PlayerCharacter/Blueprints/Actors/Bots_Parrent` _hitactor)
      (:`then`
        (if (!= (`/Game/PlayerCharacter/Blueprints/Actors/Bots_Parrent.Bot_Team_Number` _asbots_parrent) (`self.Team_Projectile_Number`))
          (if (< _distance (`self.Min_Distance_Check`))
            (set `self.Min_Distance_Check` _distance)
            (set `self.Actor_Check` _asbots_parrent))))
      (:`CastFailed`
        (bind _asmain_character (cast `/Game/PlayerCharacter/Blueprints/Main_Char/Main_Character` _hitactor))
        (if (!= (`/Game/PlayerCharacter/Blueprints/Main_Char/Main_Character.Character_Number` _asmain_character) (`self.Team_Projectile_Number`))
          (if (< _distance (`self.Min_Distance_Check`))
            (set `self.Min_Distance_Check` _distance)
            (set `self.Actor_Check` _asmain_character))))))
  (`/Engine/EditorBlueprintResources/StandardMacros.IsValid` (`self.Actor_Check`)
    (:`Is Valid`
      (`KismetSystemLibrary.Delay` 0.1)
      (goto _label :!via `Open`))))

(event `self.ReceiveTick`
  (params (DeltaSeconds :type "Float (single-precision)"))
  (`self.K2_SetActorLocation` (`KismetMathLibrary.VInterpTo_Constant` (`self.K2_GetActorLocation`) (+ (`self.K2_GetActorLocation`) (* (`SceneComponent.GetForwardVector` (`self.StaticMesh`)) (`self.Rocket_Speed_Projectile`))) DeltaSeconds 1000.0))
  (`/Engine/EditorBlueprintResources/StandardMacros.Gate` true :!label _label
    (:`Exit`
      (`SceneComponent.K2_SetWorldRotation` (`self.StaticMesh`) (`KismetMathLibrary.RInterpTo_Constant` (`SceneComponent.K2_GetComponentRotation` (`self.StaticMesh`)) (`KismetMathLibrary.FindLookAtRotation` (`self.K2_GetActorLocation`) (`self.K2_GetActorLocation` (`self.Actor_Check`))) DeltaSeconds 70.0) false false))))

(event `self.StaticMesh.OnComponentBeginOverlap`
  (params (OverlappedComponent :type "PrimitiveComponent Object Reference") (OtherActor :type "Actor Object Reference") (OtherComp :type "PrimitiveComponent Object Reference") (OtherBodyIndex :type Integer) (bFromSweep :type Boolean) (SweepResult :type "HitResult Structure (by ref)"))
  (bind (_bblockinghit _binitialoverlap _time _distance _location _impactpoint _normal _impactnormal _physmat _hitactor _hitcomponent _hitbonename _hititem _elementindex _faceindex _tracestart _traceend) (`GameplayStatics.BreakHitResult` SweepResult))
  (bind (_bblockinghit_2 _binitialoverlap_2 _time_2 _distance_2 _location_2 _impactpoint_2 _normal_2 _impactnormal_2 _physmat_2 _hitactor_2 _hitcomponent_2 _hitbonename_2 _hititem_2 _elementindex_2 _faceindex_2 _tracestart_2 _traceend_2) (`GameplayStatics.BreakHitResult` SweepResult))
  ;[1 1 1] Нанесение урона
  (`KismetSystemLibrary.Delay` 0.001)
  (bind _asbots_parrent (cast `/Game/PlayerCharacter/Blueprints/Actors/Bots_Parrent` OtherActor)
    (:`then`
      (if (!= (`self.Team_Projectile_Number`) (`/Game/PlayerCharacter/Blueprints/Actors/Bots_Parrent.Bot_Team_Number` _asbots_parrent))
        (`SceneComponent.SetHiddenInGame` (`self.StaticMesh`) true true)
        (`KismetSystemLibrary.Delay` 0.002)
        (`/Engine/EditorBlueprintResources/StandardMacros.DoOnce` false
          (:`Completed`
            (`GameplayStatics.ApplyPointDamage` _asbots_parrent (`self.Rocket_Projectile_Damage`) (`KismetMathLibrary.GetDirectionUnitVector` _traceend _tracestart) SweepResult null self)
            (`self.K2_DestroyActor`)))))
    (:`CastFailed`
      (bind _asmain_character (cast `/Game/PlayerCharacter/Blueprints/Main_Char/Main_Character` OtherActor))
      (if (!= (`self.Team_Projectile_Number`) (`/Game/PlayerCharacter/Blueprints/Main_Char/Main_Character.Character_Number` _asmain_character))
        (`SceneComponent.SetHiddenInGame` (`self.StaticMesh`) true true)
        (`KismetSystemLibrary.Delay` 0.002)
        (`/Engine/EditorBlueprintResources/StandardMacros.DoOnce` false
          (:`Completed`
            (`GameplayStatics.ApplyPointDamage` OtherActor (`self.Rocket_Projectile_Damage`) (`KismetMathLibrary.GetDirectionUnitVector` _traceend_2 _tracestart_2) SweepResult (`self.GetInstigatorController`) self)
            (`self.K2_DestroyActor`)))))))

(fn `UserConstructionScript`
  (`parent.UserConstructionScript`))